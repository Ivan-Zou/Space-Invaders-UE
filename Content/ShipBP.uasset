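; Player ship for an alien shooter, moving along X and firing projectiles from just above itself.
; The Move axis applies force to the physics collider, while Tick clamps X, pins Y to zero and kills velocity at either edge.
; Shoot spawns a PlayerProjectile with a sound.
; An overlapping AlienProjectile is destroyed with an explosion sound and takes one life from the first Global actor found in the level.
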(event `self.ReceiveTick`
  (params (DeltaSeconds :type "Float (single-precision)"))
  (bind _x (.x (`self.K2_GetActorLocation`)))
  (`self.K2_SetActorLocation` (`KismetMathLibrary.MakeVector` (`KismetMathLibrary.FClamp` (.x (`self.K2_GetActorLocation`)) -725.0 725.0) 0.0 (.z (`self.K2_GetActorLocation`))))
  (if (or (>= _x 725.0) (<= _x -725.0))
    (`PrimitiveComponent.SetAllPhysicsLinearVelocity` (`self.ShipCollider`) (0.0 0.0 0.0) false)))

(event `InputAxis|Move`
  (params (AxisValue :type "Float (single-precision)"))
  (`PrimitiveComponent.AddForce` (`self.ShipCollider`) (* (`SceneComponent.GetForwardVector` (`self.ShipCollider`)) (* AxisValue 30000.0)) "None" false))

(event `InputAction|Shoot`
  (params (Key :type "Key Structure"))
  (bind _returnvalue (`self.K2_GetActorLocation`))
  (:`Pressed`
    (`GameplayStatics.PlaySoundAtLocation` "/Game/SoundEffects/shoot.shoot" _returnvalue (struct) 1.0 1.0 0.0 null null null null)
    (`|SpawnActorFromClass` "/Game/PlayerProjectile.PlayerProjectile_C" (`KismetMathLibrary.MakeTransform` (`KismetMathLibrary.MakeVector` (.x _returnvalue) 0.0 (+ (.z _returnvalue) 35.0)) (struct :`Pitch` 90.0)) "Undefined" "OverrideRootScale" null null)))

(event `self.ShipCollider.OnComponentBeginOverlap`
  (params (OverlappedComponent :type "PrimitiveComponent Object Reference") (OtherActor :type "Actor Object Reference") (OtherComp :type "PrimitiveComponent Object Reference") (OtherBodyIndex :type Integer) (bFromSweep :type Boolean) (SweepResult :type "HitResult Structure (by ref)"))
  (cast `/Game/AlienProjectile` OtherActor)
  (`self.K2_DestroyActor` OtherActor)
  (`GameplayStatics.PlaySoundAtLocation` "/Game/SoundEffects/explosion.explosion" (`self.K2_GetActorLocation`) (struct) 1.0 1.0 0.0 null null null null)
  (bind _outactors (`GameplayStatics.GetAllActorsOfClass` "/Game/Global.Global_C"))
  (bind _output (`|GetArrayItem` _outactors))
  (set `/Game/Global.lives` (- (`/Game/Global.lives` _output) 1) _output))

(fn `UserConstructionScript`)